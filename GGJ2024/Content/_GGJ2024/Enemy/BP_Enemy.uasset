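; Enemy actor that turns to face and shoot at the player while they are inside its zone, and drops loot on death.
; Zone overlaps check BPI_PlayerRef to toggle looking and shooting.
; Tick rotates it toward player pawn 0 and calls a shoot event, where a random Delay paces projectiles fired through CompShoot.
; FNDie spawns a random pickup (tacos or coins) at its location, then destroys the enemy.
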(event `self.ReceiveTick`
  (params (DeltaSeconds :type "Float (single-precision)"))
  (if (`self.CanLook`)
    (`self.EV_LookAtPlayer`) ; Looks at Player
    (`self.EV_Shoot`) ; Shoots after Delay
  ))

(event `self.Enemy Zone Coll.OnComponentBeginOverlap`
  (params (OverlappedComponent :type "PrimitiveComponent Object Reference") (OtherActor :type "Actor Object Reference") (OtherComp :type "PrimitiveComponent Object Reference") (OtherBodyIndex :type Integer) (bFromSweep :type Boolean) (SweepResult :type "HitResult Structure (by ref)"))
  ;[1 1 1] Checks if Player is in Enemy Zone
  (if (`KismetSystemLibrary.DoesImplementInterface` OtherActor "/Game/_GGJ2024/Player/Interface/BPI_PlayerRef.BPI_PlayerRef_C")
    (set `self.CanLook` true)
    (set `self.CanShoot` true)))

(event `self.Enemy Zone Coll.OnComponentEndOverlap`
  (params (OverlappedComponent :type "PrimitiveComponent Object Reference") (OtherActor :type "Actor Object Reference") (OtherComp :type "PrimitiveComponent Object Reference") (OtherBodyIndex :type Integer))
  ;[1 1 1] Checks if Player is in Enemy Zone
  (if (`KismetSystemLibrary.DoesImplementInterface` OtherActor "/Game/_GGJ2024/Player/Interface/BPI_PlayerRef.BPI_PlayerRef_C")
    (set `self.CanLook` false)
    (set `self.CanShoot` false)))

(event `EV_Shoot`
  ;[1 1 1] Shoot Event
  (if (`self.CanShoot`)
    (`KismetSystemLibrary.Delay` (`KismetArrayLibrary.Array_Random` (`self.ShootingDelay`)))
    (`/Game/_GGJ2024/Player/Components/Comp_Shoot.FN_Shoot` (`self.Comp_Shoot`) "/Game/_GGJ2024/Enemy/BP_EnemyProjectile.BP_EnemyProjectile_C" (`self.Shooting Point`)) ; Shoots Player
  ))

(event `/Game/_GGJ2024/Player/Interface/BPI_Die.FN_Die`
  ;[1 1 1] Death Event
  (`|SpawnActorFromClass` (`KismetArrayLibrary.Array_Random` (`self.Class`)) (`KismetMathLibrary.Conv_VectorToTransform` (`self.K2_GetActorLocation`)) "Undefined" "MultiplyWithRoot" null null)
  (`self.K2_DestroyActor`))

(fn `EV_LookAtPlayer`
  (`self.K2_SetActorRotation` (`KismetMathLibrary.FindLookAtRotation` (`self.K2_GetActorLocation`) (`self.K2_GetActorLocation` (`GameplayStatics.GetPlayerPawn` 0)))))

(fn `UserConstructionScript`)