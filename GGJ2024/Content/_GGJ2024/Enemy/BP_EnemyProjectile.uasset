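; Enemy projectile actor that damages the player when its sphere hits an actor implementing BPI_PlayerRef.
; On such a hit, it gets the player reference through the interface, applies BaseDamage to it and destroys itself.
; A one-second Delay on Tick serves as the lifetime, destroying the projectile if it has not hit by then.
; Debug strings report hits and misses.
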(event `self.ReceiveTick`
  (params (DeltaSeconds :type "Float (single-precision)"))
  (`KismetSystemLibrary.Delay` 1.0)
  (`self.K2_DestroyActor`)
  (`KismetSystemLibrary.PrintString` "NOT HIT!"))

(event `self.Sphere.OnComponentHit`
  (params (HitComponent :type "PrimitiveComponent Object Reference") (OtherActor :type "Actor Object Reference") (OtherComp :type "PrimitiveComponent Object Reference") (NormalImpulse :type "Vector Structure") (Hit :type "HitResult Structure (by ref)"))
  (if (`KismetSystemLibrary.DoesImplementInterface` OtherActor "/Game/_GGJ2024/Player/Interface/BPI_PlayerRef.BPI_PlayerRef_C")
    (bind _playerref (message `/Game/_GGJ2024/Player/Interface/BPI_PlayerRef.FN_PlayerRef` OtherActor))
    (`GameplayStatics.ApplyDamage` _playerref (`self.Base Damage`))
    (`self.K2_DestroyActor`)
    (`KismetSystemLibrary.PrintString` "HIT!")))

(fn `UserConstructionScript`)