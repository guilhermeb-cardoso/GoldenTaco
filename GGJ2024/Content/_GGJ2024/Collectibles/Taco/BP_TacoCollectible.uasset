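; Taco pickup that spins in place and homes in on the player in a game-jam project (GGJ2024).
; Tick adds yaw each frame and, when the player pawn is within range, waits briefly, then plays a timeline that lerps the taco toward the pawn.
; Sphere overlap with an actor implementing BPI_PlayerRef sends a gain-tacos message, plays a sound and destroys the pickup.
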(event `self.ReceiveTick`
  (params (DeltaSeconds :type "Float (single-precision)"))
  (bind (_returnvalue_roll _returnvalue_pitch _returnvalue_yaw) (`KismetMathLibrary.BreakRotator` (`self.K2_GetActorRotation`)))
  (`self.K2_SetActorRotation` (`KismetMathLibrary.MakeRotator` _returnvalue_roll _returnvalue_pitch (+ _returnvalue_yaw (`self.RotationSpeed`))))
  (if (<= (`KismetMathLibrary.Vector_Distance` (`self.K2_GetActorLocation`) (`self.K2_GetActorLocation` (`GameplayStatics.GetPlayerPawn` 0))) 600.0)
    (`KismetSystemLibrary.Delay` 0.4)
    (bind (_direction _newtrack_0) (`Timeline|Timeline`)
      (:`Update`
        (`self.K2_SetActorRelativeLocation` (`KismetMathLibrary.VLerp` (`self.K2_GetActorLocation`) (`self.K2_GetActorLocation` (`GameplayStatics.GetPlayerPawn` 0)) _newtrack_0) true)))))

(event `self.Sphere.OnComponentBeginOverlap`
  (params (OverlappedComponent :type "PrimitiveComponent Object Reference") (OtherActor :type "Actor Object Reference") (OtherComp :type "PrimitiveComponent Object Reference") (OtherBodyIndex :type Integer) (bFromSweep :type Boolean) (SweepResult :type "HitResult Structure (by ref)"))
  (if (`KismetSystemLibrary.DoesImplementInterface` OtherActor "/Game/_GGJ2024/Player/Interface/BPI_PlayerRef.BPI_PlayerRef_C")
    (bind _playerref (message `/Game/_GGJ2024/Player/Interface/BPI_PlayerRef.FN_PlayerRef` OtherActor))
    (message `/Game/_GGJ2024/Player/Interface/BPI_PlayerRef.FN_GainTacos` _playerref)
    (`GameplayStatics.PlaySoundAtLocation` "/Engine/VREditor/Sounds/UI/Camera_Shutter.Camera_Shutter" (`self.K2_GetActorLocation`) (struct) 1.0 1.0 0.0 null null null null)
    (`self.K2_DestroyActor`)))

(fn `UserConstructionScript`)