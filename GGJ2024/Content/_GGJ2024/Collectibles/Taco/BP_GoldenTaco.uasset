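; BP_GoldenTaco is a collectible golden taco that wins the game when the player interacts with it.
; Tick spins the actor and turns its PressE prompt toward the player, hiding the prompt beyond a set distance.
; A sphere overlap with any Character enables or disables the actor's input.
; Pressing E plays a burst of camera-shutter sounds with short delays, then opens the YouWon level.
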(event `self.ReceiveTick`
  (params (DeltaSeconds :type "Float (single-precision)"))
  (bind (_returnvalue_roll _returnvalue_pitch _returnvalue_yaw) (`KismetMathLibrary.BreakRotator` (`self.K2_GetActorRotation`)))
  (bind _presse (`self.PressE`))
  (`self.K2_SetActorRotation` (`KismetMathLibrary.MakeRotator` _returnvalue_roll _returnvalue_pitch (+ _returnvalue_yaw 1.5)))
  (`SceneComponent.K2_SetWorldRotation` (`self.PressE`) (`KismetMathLibrary.FindLookAtRotation` (`self.K2_GetActorLocation`) (`self.K2_GetActorLocation` (`GameplayStatics.GetPlayerPawn` 0))) false false) ; Makes so the Text is Always \nturned Towards the player
  (if (> (`self.GetDistanceTo` (`GameplayStatics.GetPlayerPawn` 0)) 1000.0)
    (`SceneComponent.SetVisibility` _presse false false) ; Invisible
    (else
      (`SceneComponent.SetVisibility` _presse true false) ; Visible
    )))

(event `self.Sphere.OnComponentBeginOverlap`
  (params (OverlappedComponent :type "PrimitiveComponent Object Reference") (OtherActor :type "Actor Object Reference") (OtherComp :type "PrimitiveComponent Object Reference") (OtherBodyIndex :type Integer) (bFromSweep :type Boolean) (SweepResult :type "HitResult Structure (by ref)"))
  (bind _ascharacter (cast `Character` OtherActor))
  (`/Engine/EditorBlueprintResources/StandardMacros.IsValid` _ascharacter
    (:`Is Valid`
      (`self.EnableInput` (`GameplayStatics.GetPlayerController` 0)))))

(event `self.Sphere.OnComponentEndOverlap`
  (params (OverlappedComponent :type "PrimitiveComponent Object Reference") (OtherActor :type "Actor Object Reference") (OtherComp :type "PrimitiveComponent Object Reference") (OtherBodyIndex :type Integer))
  (bind _ascharacter (cast `Character` OtherActor))
  (`/Engine/EditorBlueprintResources/StandardMacros.IsValid` _ascharacter
    (:`Is Valid`
      (`self.DisableInput` (`GameplayStatics.GetPlayerController` 0)))))

(event `EV_YouWon`
  (`GameplayStatics.PlaySound2D` "/Engine/VREditor/Sounds/UI/Camera_Shutter.Camera_Shutter" 1.0 1.0 0.0 null null)
  (`KismetSystemLibrary.Delay` 0.2)
  (`GameplayStatics.PlaySound2D` "/Engine/VREditor/Sounds/UI/Camera_Shutter.Camera_Shutter" 1.0 1.0 0.0 null null)
  (`KismetSystemLibrary.Delay` 0.2)
  (`GameplayStatics.PlaySound2D` "/Engine/VREditor/Sounds/UI/Camera_Shutter.Camera_Shutter" 1.0 1.0 0.0 null null)
  (`KismetSystemLibrary.Delay` 0.5)
  (`GameplayStatics.OpenLevel` "YouWon"))

(event `Key|E`
  (params (Key :type "Key Structure"))
  (:`Pressed`
    (`self.EV_YouWon`)))

(fn `UserConstructionScript`)