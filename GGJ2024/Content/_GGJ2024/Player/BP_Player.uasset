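; BP_Player is the player character, with Enhanced Input movement, look, jump and shooting, plus a pause menu toggled by Escape or P.
; Shooting fires BP_Projectile through CompShoot, with timeline-driven mesh recoil and a throttled Niagara muzzle effect.
; A health check on Tick converts collected coins and tacos into capped CompHealth health and opens the GameOver level at zero health.
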(event `self.ReceiveBeginPlay`
  (`|ExecutionSequence`
    (:`then_0`
      ;[1 1 1] Gets Controls
      (bind _asbp_player_controller (cast `/Game/_GGJ2024/Player/Controls/BP_PlayerController` (`GameplayStatics.GetPlayerController` 0)))
      (bind _returnvalue (pcsubsystem `EnhancedInputLocalPlayerSubsystem` _asbp_player_controller))
      (`/Engine/EditorBlueprintResources/StandardMacros.IsValid` _returnvalue
        (:`Is Valid`
          (`EnhancedInputSubsystemInterface.AddMappingContext` _returnvalue "/Game/_GGJ2024/Player/Controls/IMC_Player.IMC_Player" 0 (struct)))))
    (:`then_1`
      ;[1 1 1] Player's HP
      (set `/Game/_GGJ2024/Player/Components/Comp_Health.Health` (`self.Health`) (`self.Comp_Health`)))
    (:`then_2`
      (if (>= (`/Game/_GGJ2024/Player/Components/Comp_Health.Health` (`self.Comp_Health`)) 10.0)
        (bind _output_get (set `/Game/_GGJ2024/Player/Components/Comp_Health.Health` 10.0 (`self.Comp_Health`)))
        (`KismetSystemLibrary.PrintString` (`KismetStringLibrary.Conv_DoubleToString` _output_get))))))

(event `self.ReceiveTick`
  (params (DeltaSeconds :type "Float (single-precision)"))
  ;[1 1 1] Updates Health
  (`self.EV_HealthSystem`)
  (`KismetSystemLibrary.PrintString` (`KismetStringLibrary.Conv_DoubleToString` (`/Game/_GGJ2024/Player/Components/Comp_Health.Health` (`self.Comp_Health`))) true true (struct :`R` 1.0 :`B` 0.005 :`A` 1.0) 0.0))

(event `EnhancedInput|/Game/_GGJ2024/Player/Controls/IA_JumpGGJ`
  (params (ActionValue :type Boolean) (ElapsedSeconds :type "Float (double-precision)") (TriggeredSeconds :type "Float (double-precision)") (InputAction :type "InputAction Object Reference" :default "/Game/_GGJ2024/Player/Controls/IA_JumpGGJ.IA_JumpGGJ"))
  ;[1 1 1] Jump Controls
  (:`Started`
    (`self.Jump`))
  (:`Completed`
    (`self.StopJumping`)))

(event `EnhancedInput|/Game/_GGJ2024/Player/Controls/IA_LookGGJ`
  (params (ActionValue :type "Vector2D Structure") (ElapsedSeconds :type "Float (double-precision)") (TriggeredSeconds :type "Float (double-precision)") (InputAction :type "InputAction Object Reference" :default "/Game/_GGJ2024/Player/Controls/IA_LookGGJ.IA_LookGGJ"))
  ;[1 1 1] Look Controls
  (:`Triggered`
    (`self.AddControllerYawInput` ActionValue_X) ; Left/Right
    (bind _result (`/Engine/EditorBlueprintResources/StandardMacros.NegateFloat` ActionValue_Y) ; Negate Float so  it Inverts \nUP/Down Values
      (:`  `
        (`self.AddControllerPitchInput` _result) ; UP/DOWN
      ))))

(event `EnhancedInput|/Game/_GGJ2024/Player/Controls/IA_MovementGGJ`
  (params (ActionValue :type "Vector2D Structure") (ElapsedSeconds :type "Float (double-precision)") (TriggeredSeconds :type "Float (double-precision)") (InputAction :type "InputAction Object Reference" :default "/Game/_GGJ2024/Player/Controls/IA_MovementGGJ.IA_MovementGGJ"))
  ;[1 1 1] Movement Controls
  (:`Triggered`
    (`self.AddMovementInput` (`self.GetActorForwardVector`) ActionValue_X)
    (`self.AddMovementInput` (`self.GetActorRightVector`) ActionValue_Y)))

(event `EnhancedInput|/Game/_GGJ2024/Player/Controls/IA_ShootGGJ`
  (params (ActionValue :type Boolean) (ElapsedSeconds :type "Float (double-precision)") (TriggeredSeconds :type "Float (double-precision)") (InputAction :type "InputAction Object Reference" :default "/Game/_GGJ2024/Player/Controls/IA_ShootGGJ.IA_ShootGGJ"))
  (bind _skeletalmesh (`self.SkeletalMesh`))
  (bind (_relativelocation_x _relativelocation_y _relativelocation_z) (`KismetMathLibrary.BreakVector` (`SceneComponent.RelativeLocation` _skeletalmesh)))
  ;[1 1 1] Shooting Controls
  (:`Triggered`
    (`/Game/_GGJ2024/Player/Components/Comp_Shoot.FN_Shoot` (`self.Comp_Shoot`) "/Game/_GGJ2024/Player/BP_Projectile.BP_Projectile_C" (`self.Shooting Direction`))
    (bind (_direction _newtrack_0) (`Timeline|TL_ShotAnim` :!via `PlayFromStart`)
      (:`Update`
        (`SceneComponent.K2_SetRelativeLocation` _skeletalmesh (`KismetMathLibrary.MakeVector` (`KismetMathLibrary.Lerp` 20.0 18.0 _newtrack_0) _relativelocation_y _relativelocation_z) true false)
        (`/Engine/EditorBlueprintResources/StandardMacros.Do N` 1 :!label _label ; Executes Code N Amount of Times
          (:`Exit`
            (`NiagaraFunctionLibrary.SpawnSystemAtLocation` "/Game/_GGJ2024/Player/FX/NS_GunShotFx.NS_GunShotFx" (`SceneComponent.K2_GetComponentLocation` (`self.Shooting Direction`)))
            (`KismetSystemLibrary.Delay` 0.3)
            (goto _label :!via `Reset`)))))))

(event `/Game/_GGJ2024/Player/Interface/BPI_Die.FN_Die`
  ;[1 1 1] Dying Function
  (`GameplayStatics.OpenLevel` "GameOver") ; Game Over Level
)

(event `/Game/_GGJ2024/Player/Interface/BPI_PlayerRef.FN_GainCoin`
  (bind _coins (`self.Coins`))
  (bind _result (`/Engine/EditorBlueprintResources/StandardMacros.IncrementInt` _coins)
    (:`  `
      (set `self.Coins` _result)
      (`KismetSystemLibrary.PrintString` (`KismetStringLibrary.Concat_StrStr` "Coins" (`KismetStringLibrary.Conv_IntToString` _coins))))))

(event `/Game/_GGJ2024/Player/Interface/BPI_PlayerRef.FN_GainTacos`
  ;[1 1 1] Gain Tacos Function
  (bind _result (`/Engine/EditorBlueprintResources/StandardMacros.IncrementInt` (`self.Tacos`))
    (:`  `
      (bind _output_get (set `self.Tacos` _result))
      (`KismetSystemLibrary.PrintString` (`KismetStringLibrary.Concat_StrStr` "Tacos" (`KismetStringLibrary.Conv_IntToString` _output_get))))))

(event `EV_HealthSystem`
  (bind _comp_health (`self.Comp_Health`))
  (bind _comp_health_2 (`self.Comp_Health`))
  ;[1 1 1] Health System Event
  (`|ExecutionSequence`
    (:`then_0`
      (if (== (`self.Coins`) 10)
        (bind _output_get (set `/Game/_GGJ2024/Player/Components/Comp_Health.Health` (+ (`/Game/_GGJ2024/Player/Components/Comp_Health.Health` _comp_health_2) 1.0) _comp_health_2))
        (set `self.Coins` 0)
        (`KismetSystemLibrary.PrintString` (`KismetStringLibrary.Conv_DoubleToString` _output_get))))
    (:`then_1`
      (if (== (`self.Tacos`) 5)
        (set `/Game/_GGJ2024/Player/Components/Comp_Health.Health` (+ (`/Game/_GGJ2024/Player/Components/Comp_Health.Health` _comp_health) 1.0) _comp_health)
        (set `self.Tacos` 0)
        (`KismetSystemLibrary.PrintString` (`KismetStringLibrary.Conv_DoubleToString` 0.0))))
    (:`then_2`
      (if (>= (`/Game/_GGJ2024/Player/Components/Comp_Health.Health` (`self.Comp_Health`)) 10.0)
        (set `/Game/_GGJ2024/Player/Components/Comp_Health.Health` 10.0 (`self.Comp_Health`))))
    (:`then_3`
      (if (<= (`/Game/_GGJ2024/Player/Components/Comp_Health.Health` (`self.Comp_Health`)) 0.0)
        (`self.FN_Die`)))))

(event `Key|Escape` :paused true
  (params (Key :type "Key Structure"))
  (bind _returnvalue (`GameplayStatics.GetPlayerController` 0))
  (bind _returnvalue_2 (`GameplayStatics.GetPlayerController` 0))
  ;[1 1 1] Pause
  (:`Pressed`
    (`/Engine/EditorBlueprintResources/StandardMacros.FlipFlop` :!label _label_2
      (:`A`
        (`GameplayStatics.SetGamePaused` true)
        (set `PlayerController.bShowMouseCursor` true _returnvalue)
        (`WidgetBlueprintLibrary.SetInputMode_GameOnly` _returnvalue_2 true)
        (bind _returnvalue_3 (`|CreateWidget` "/Game/_GGJ2024/Menus/Pause/WBP_PauseMenu.WBP_PauseMenu_C"))
        (`UserWidget.AddToViewport` _returnvalue_3 0))
      (:`B`
        (`GameplayStatics.SetGamePaused` false)
        (set `PlayerController.bShowMouseCursor` false _returnvalue)
        (`WidgetBlueprintLibrary.SetInputMode_GameOnly` _returnvalue_2 true)
        (`Widget.RemoveFromParent` _returnvalue_3)))))

(event `Key|P` :paused true
  (params (Key :type "Key Structure"))
  ;[1 1 1] Pause
  (:`Pressed`
    (goto _label_2)))

(fn `FN_PlayerRef`
  (returns (PlayerRef :type "Character Object Reference"))
  (return self))

(fn `UserConstructionScript`)