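; BP_Saw is a spinning saw hazard that knocks the player back and damages them on contact.
; Tick rotates the static mesh by a fixed step each frame, independent of delta time.
; When an actor implementing BPI_PlayerRef overlaps the Box, player character 0 is launched opposite its facing direction and the overlapping actor takes damage.
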(event `self.ReceiveTick`
  (params (DeltaSeconds :type "Float (single-precision)"))
  (`SceneComponent.K2_AddLocalRotation` (`self.StaticMesh`) (struct :`Pitch` -1.0) false false))

(event `self.Box.OnComponentBeginOverlap`
  (params (OverlappedComponent :type "PrimitiveComponent Object Reference") (OtherActor :type "Actor Object Reference") (OtherComp :type "PrimitiveComponent Object Reference") (OtherBodyIndex :type Integer) (bFromSweep :type Boolean) (SweepResult :type "HitResult Structure (by ref)"))
  (bind _returnvalue (`GameplayStatics.GetPlayerCharacter` 0))
  (if (`KismetSystemLibrary.DoesImplementInterface` OtherActor "/Game/_GGJ2024/Player/Interface/BPI_PlayerRef.BPI_PlayerRef_C")
    (`Character.LaunchCharacter` _returnvalue (* (`KismetMathLibrary.GetForwardVector` (`self.K2_GetActorRotation` _returnvalue)) (-2000.0 -2000.0 -2000.0)) false false)
    (`GameplayStatics.ApplyDamage` OtherActor 1.0)))

(fn `UserConstructionScript`)