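; BP_RespawnColl is a trigger volume that sends the player back to the respawn point at a health cost.
; On Box overlap by a BP_Player with health above zero, it teleports player pawn 0 to the RespawnPoint stored in BP_FirstPersonGameMode.
; It then decrements CompHealth.Health on the BP_Player found through GetActorOfClass, rather than on the overlapping actor reference.
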(event `self.Box.OnComponentBeginOverlap`
  (params (OverlappedComponent :type "PrimitiveComponent Object Reference") (OtherActor :type "Actor Object Reference") (OtherComp :type "PrimitiveComponent Object Reference") (OtherBodyIndex :type Integer) (bFromSweep :type Boolean) (SweepResult :type "HitResult Structure (by ref)"))
  (bind _asbp_player (cast `/Game/_GGJ2024/Player/BP_Player` OtherActor))
  (`/Engine/EditorBlueprintResources/StandardMacros.IsValid` _asbp_player
    (:`Is Valid`
      (bind _asbp_first_person_game_mode (cast `/Game/FirstPerson/Blueprints/BP_FirstPersonGameMode` (`GameplayStatics.GetGameMode`)))
      (`/Engine/EditorBlueprintResources/StandardMacros.IsValid` _asbp_first_person_game_mode
        (:`Is Valid`
          (if (> (`/Game/_GGJ2024/Player/Components/Comp_Health.Health` (`/Game/_GGJ2024/Player/BP_Player.Comp_Health` _asbp_player)) 0.0)
            (bind (_respawnpoint_location _respawnpoint_rotation) (`KismetMathLibrary.BreakTransform` (`/Game/FirstPerson/Blueprints/BP_FirstPersonGameMode.RespawnPoint` _asbp_first_person_game_mode)))
            (`self.K2_TeleportTo` (`GameplayStatics.GetPlayerPawn` 0) _respawnpoint_location _respawnpoint_rotation)
            (bind _returnvalue (`GameplayStatics.GetActorOfClass` "/Game/_GGJ2024/Player/BP_Player.BP_Player_C"))
            (`/Engine/EditorBlueprintResources/StandardMacros.DecrementFloat` (`/Game/_GGJ2024/Player/Components/Comp_Health.Health` (`/Game/_GGJ2024/Player/BP_Player.Comp_Health` _returnvalue)))))))))

(fn `UserConstructionScript`)